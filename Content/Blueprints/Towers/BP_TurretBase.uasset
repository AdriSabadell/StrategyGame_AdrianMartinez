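; Base tower turret that tracks one enemy and fires bullets at it.
; ShootRadius overlaps lock the first entering BP_EnemyBase as target and clear it on exit, without searching for others already in range.
; A looping timer yaw-rotates Axis toward the target and spawns a BP_BulletBase at ShootPoint, passing speed, damage and target to it.
; SetShootSpeed restarts that timer with a new interval but does not store the new handle.
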(event `self.ReceiveBeginPlay`
  (bind _returnvalue (`KismetSystemLibrary.K2_SetTimerDelegate` (delegate `TurretTick`) (`self.GetShootSpeed`) true))
  (set `self.mTickHandler` _returnvalue))

(event `SetShootSpeed`
  (params (aShootSpeed :type "Float (double-precision)"))
  (`KismetSystemLibrary.K2_InvalidateTimerHandle` (`self.mTickHandler`))
  (bind _output_get (set `self.mShootSpeed` (/ 1.0 aShootSpeed)))
  (`KismetSystemLibrary.K2_SetTimerDelegate` (delegate `TurretTick`) _output_get true))

(event `TurretTick`
  (`self.RotateToEnemy`)
  (`self.mTarget`
    (:`then`
      (bind _returnvalue (`|SpawnActorFromClass` "/Game/Blueprints/Towers/BP_BulletBase.BP_BulletBase_C" (`SceneComponent.K2_GetComponentToWorld` (`self.ShootPoint`)) "AlwaysSpawn" "MultiplyWithRoot" null (`self.mBulletSpeed`) (`self.mBulletDamage`) null))
      (set `/Game/Blueprints/Components/BPC_MoveToTarget.mTarget` (`self.mTarget`) (`/Game/Blueprints/Towers/BP_BulletBase.BPC_MoveToTarget` _returnvalue))
      (`KismetSystemLibrary.PrintString` "SpawneaBala"))
    (:`else`)))

(event `self.ShootRadius.OnComponentBeginOverlap`
  (params (OverlappedComponent :type "PrimitiveComponent Object Reference") (OtherActor :type "Actor Object Reference") (OtherComp :type "PrimitiveComponent Object Reference") (OtherBodyIndex :type Integer) (bFromSweep :type Boolean) (SweepResult :type "HitResult Structure (by ref)"))
  (bind _asbp_enemy_base (cast `/Game/Blueprints/Enemies/BP_EnemyBase` OtherActor))
  (`self.mTarget`
    (:`then`)
    (:`else`
      (set `self.mTarget` _asbp_enemy_base)
      (`KismetSystemLibrary.PrintString` "Entra enemigo" true true (struct :`R` 1.0 :`G` 0.16801 :`A` 1.0)))))

(event `self.ShootRadius.OnComponentEndOverlap`
  (params (OverlappedComponent :type "PrimitiveComponent Object Reference") (OtherActor :type "Actor Object Reference") (OtherComp :type "PrimitiveComponent Object Reference") (OtherBodyIndex :type Integer))
  (bind _asbp_enemy_base (cast `/Game/Blueprints/Enemies/BP_EnemyBase` OtherActor))
  (if (== _asbp_enemy_base (`self.mTarget`))
    (set `self.mTarget` null)
    (`KismetSystemLibrary.PrintString` "Sale enemigo" true true (struct :`R` 0.212236 :`G` 1.0 :`A` 1.0))))

(fn `GetShootSpeed`
  (returns (ReturnValue :type "Float (double-precision)"))
  (return (/ 1.0 (`self.mShootSpeed`))))

(fn `RotateToEnemy`
  (bind _mtarget (`self.mTarget`)
    (:`then`
      (bind (_x _y) (`KismetMathLibrary.BreakVector3f` (`KismetMathLibrary.BreakRotIntoAxes` (`KismetMathLibrary.FindLookAtRotation` (`SceneComponent.K2_GetComponentLocation` (`self.Axis`)) (`self.K2_GetActorLocation` _mtarget)))))
      (`SceneComponent.K2_SetRelativeRotation` (`self.Axis`) (`KismetMathLibrary.MakeRotationFromAxes` (`KismetMathLibrary.MakeVector` _x _y)) false false))
    (:`else`)))

(fn `UserConstructionScript`)