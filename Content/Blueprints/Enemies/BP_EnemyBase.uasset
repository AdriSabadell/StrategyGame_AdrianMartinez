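; Base enemy that follows a waypoint path and can be killed by damage.
; On BeginPlay it spawns its default controller and runs Tracking, which chains AI MoveTo calls through the waypoint array and destroys the enemy after the last one.
; Any damage lowers health and replays the Blink timeline, which drives a material parameter on the cube as a hit flash.
; At zero health it sets a short lifespan once.
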(event `self.ReceiveBeginPlay`
  (`|ExecutionSequence`
    (:`then_0`
      (`self.SpawnDefaultController`)
      (`self.Tracking`))
    (:`then_1`
      (add `self.OnTakeAnyDamage` (delegate `OnTakeAnyDamage_Event`)))))

(event `OnTakeAnyDamage_Event` :!signature `self.OnTakeAnyDamage`
  (params (DamagedActor :type "Actor Object Reference") (Damage :type "Float (single-precision)") (DamageType :type "DamageType Object Reference") (InstigatedBy :type "Controller Object Reference") (DamageCauser :type "Actor Object Reference"))
  (bind _output_get (set `self.mHealthPoints` (- (`self.mHealthPoints`) Damage)))
  (`KismetSystemLibrary.PrintString` (`KismetStringLibrary.Conv_DoubleToString` _output_get))
  (if (<= _output_get 0.0)
    (`/Engine/EditorBlueprintResources/StandardMacros.DoOnce` false
      (:`Completed`
        (`self.SetLifeSpan` 0.5))))
  (`TimelineComponent.SetPlayRate` (`self.Blink`) 1.0)
  (bind (_direction _blinkvaue) (`Timeline|Blink` :!via `PlayFromStart`)
    (:`Update`
      (`MeshComponent.SetScalarParameterValueOnMaterials` (`self.Cube`) "Blink" _blinkvaue))))

(event `Tracking`
  (bind _movementresult (`|AIMoveTo` self (0.0 0.0 0.0) (`|GetArrayItem` (`self.mWaypoints`) (`self.mCurrWaypointIndex`)))
    (:`OnSuccess`
      (bind _result (`/Engine/EditorBlueprintResources/StandardMacros.IncrementInt` (`self.mCurrWaypointIndex`))
        (:`  `
          (if (>= _result (`KismetArrayLibrary.Array_Length` (`self.mWaypoints`)))
            (`KismetSystemLibrary.PrintString` "Muerte" true true (struct :`R` 1.0 :`B` 0.127223 :`A` 1.0))
            (`self.K2_DestroyActor`)
            (else
              (`KismetSystemLibrary.PrintString` "Siguiente" true true (struct :`R` 0.896367 :`B` 1.0 :`A` 1.0))
              (`self.Tracking`))))))
    (:`OnFail`
      (`KismetSystemLibrary.PrintString` (`|GetEnumeratorNameAsString` _movementresult)))))

(fn `UserConstructionScript`)