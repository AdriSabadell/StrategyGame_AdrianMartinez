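; Enemy spawner actor that runs a sequence of timed waves, starting shortly after BeginPlay.
; StartWave spawns each enemy class listed in the current Waves entry at the spawner's transform, passing it MWaypoints and pausing by that wave's InBetweenTime.
; When a wave's list runs out, it waits briefly and calls itself with the next index.
; After the last wave, it only prints an end message.
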(event `self.ReceiveBeginPlay`
  (`KismetSystemLibrary.Delay` 3.0)
  (`self.StartWave` 0))

(event `StartWave`
  (params (NewParam :type Integer))
  (bind (_inbetweentime _enemies) (break `/Game/Blueprints/Enemies/Waves/WaveStruct` (`|GetArrayItem` (`self.Waves`) NewParam)))
  (if (`KismetArrayLibrary.Array_IsValidIndex` (`self.Waves`) NewParam)
    (bind _output_get (set `self.EnemyIndex` 0))
    (if (`KismetArrayLibrary.Array_IsValidIndex` _enemies _output_get) :!label _label
      ;[0.5473 0.1145 1] Create enemy from Wave
      (`|SpawnActorFromClass` (`|GetArrayItem` _enemies _output_get) (`self.GetTransform`) "Undefined" "MultiplyWithRoot" null (`self.mWaypoints`) null)
      (`/Engine/EditorBlueprintResources/StandardMacros.IncrementInt` (`self.EnemyIndex`)
        (:`  `
          (`KismetSystemLibrary.Delay` _inbetweentime)
          (goto _label)))
      (else
        ;[1 0 0] NextWave
        (`KismetSystemLibrary.Delay` 3.0)
        (`self.StartWave` (+ NewParam 1))))
    (else
      ;[1 0.9408 0] End Wave
      (`KismetSystemLibrary.PrintString` "EndWaves"))))

(fn `UserConstructionScript`)