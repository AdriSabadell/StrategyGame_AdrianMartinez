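; Player controller that handles mouse-driven turret placement through a None, Choosing, Building and Built state machine.
; Right click toggles the turret menu via a dispatcher, and a HUD button stores the turret ID and starts Building.
; Each tick while Building, a cursor trace updates the placement point, ignoring turret and path hits.
; Left click confirms, and the next tick spawns BP_TurretBase there regardless of the stored ID.
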(event `self.ReceiveBeginPlay`
  ;[1 1 1] Start
  (bind _asgmbbp (cast `/Game/GMBBP` (`GameplayStatics.GetGameMode`)))
  (set `self.mGameMode` _asgmbbp)
  (`EnhancedInputSubsystemInterface.AddMappingContext` (subsystem `EnhancedInputLocalPlayerSubsystem`) "/Game/Blueprints/Inputs/IMC_Base.IMC_Base" 0 (struct))
  (`GameplayStatics.SetViewportMouseCaptureMode` "CapturePermanently_IncludingInitialMouseDown")
  (bind _asbp_player_character (cast `/Game/Blueprints/Player/BP_PlayerCharacter` (`GameplayStatics.GetPlayerCharacter` 0)))
  (set `self.mPlayerCharacter` _asbp_player_character))

(event `EnhancedInput|/Game/Blueprints/Inputs/IA_LeftClick`
  (params (ActionValue :type Boolean) (ElapsedSeconds :type "Float (double-precision)") (TriggeredSeconds :type "Float (double-precision)") (InputAction :type "InputAction Object Reference" :default "/Game/Blueprints/Inputs/IA_LeftClick.IA_LeftClick"))
  ;[1 1 1 1 34] MouseInputs
  (:`Started`
    (switch `/Game/Blueprints/Player/EBuildingState` (`self.mBuildingState`)
      (:`NewEnumerator1`
        (`self.OnOpenTurretMenu` false)
        (set `self.mBuildingState` "NewEnumerator3")))))

(event `EnhancedInput|/Game/Blueprints/Inputs/IA_RightClick`
  (params (ActionValue :type Boolean) (ElapsedSeconds :type "Float (double-precision)") (TriggeredSeconds :type "Float (double-precision)") (InputAction :type "InputAction Object Reference" :default "/Game/Blueprints/Inputs/IA_RightClick.IA_RightClick"))
  ;[1 1 1 1 34] MouseInputs
  (:`Started`
    (switch `/Game/Blueprints/Player/EBuildingState` (`self.mBuildingState`)
      (:`NewEnumerator0`
        (`self.OnOpenTurretMenu` true)
        (set `self.mBuildingState` "NewEnumerator2"))
      (:`NewEnumerator2`
        (`self.OnOpenTurretMenu` false)
        (set `self.mBuildingState` "NewEnumerator0")))))

(event `self.ReceiveTick`
  (params (DeltaSeconds :type "Float (single-precision)"))
  (switch `/Game/Blueprints/Player/EBuildingState` (`self.mBuildingState`)
    (:`NewEnumerator1`
      (`self.PreviewBuilding`))
    (:`NewEnumerator3`
      (`|SpawnActorFromClass` "/Game/Blueprints/Towers/BP_TurretBase.BP_TurretBase_C" (`KismetMathLibrary.Conv_VectorToTransform` (`self.mMousePos`)) "Undefined" "MultiplyWithRoot" null null)
      (set `self.mBuildingState` "NewEnumerator0"))))

(event `PreviewBuilding`
  (bind (_worldlocation _worlddirection) (`self.DeprojectMousePositionToWorld`))
  (bind _returnvalue_location (`KismetMathLibrary.BreakTransform` (`SceneComponent.K2_GetComponentToWorld` (`/Game/Blueprints/Player/BP_PlayerCharacter.PlayerCamera` (`self.mPlayerCharacter`)))))
  (bind _outhit (`KismetSystemLibrary.LineTraceSingle` :`Start` _returnvalue_location :`End` (+ _worldlocation (* _worlddirection 3500.0)) :`TraceChannel` "TraceTypeQuery1" :`DrawDebugType` "Persistent"))
  (`|ExecutionSequence`
    (:`then_1`
      (bind (_bblockinghit _binitialoverlap _time _distance _location _impactpoint _normal _impactnormal _physmat _hitactor) (`GameplayStatics.BreakHitResult` _outhit))
      (cast `/Game/Blueprints/Towers/BP_TurretBase` _hitactor
        (:`CastFailed`
          (cast `/Game/Blueprints/Towers/BP_Path` _hitactor
            (:`CastFailed`
              (set `self.mMousePos` _impactpoint))))))))

(event `HUDButtonPressed`
  (params (aTurretID :type "/Game/Blueprints/Towers/eTurrets Enum" :default "NewEnumerator0"))
  (set `self.mTurretToBuild` aTurretID)
  (set `self.mBuildingState` "NewEnumerator1"))

(fn `UserConstructionScript`)